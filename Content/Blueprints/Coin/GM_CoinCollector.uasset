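; Game mode for a coin collecting game that tracks collected coins against the level's total.
; On BeginPlay it spawns a coin at every coin spawn actor, sums those with the coins held in treasure chests, and adds the coin counter widget to the viewport.
; CollectCoin and LootChest raise the count, update the widget and print whether all coins are found.
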(event `self.ReceiveBeginPlay`
  (`|ExecutionSequence`
    (:`then_0`
      ;[1 1 1] Instantiate Coins on every coin Spawn actor
      (bind _outactors (`GameplayStatics.GetAllActorsOfClass` "/Game/Blueprints/Coin/BP_CoinSpawn.BP_CoinSpawn_C"))
      (set `self.MaxCoinCount` (`KismetArrayLibrary.Array_Length` _outactors))
      (for _array_element _outactors
        (`|SpawnActorFromClass` "/Game/Blueprints/Coin/BP_Coin.BP_Coin_C" (`self.GetTransform` _array_element) "Undefined" "OverrideRootScale" null null)))
    (:`then_1`
      ;[1 1 1] Get Coins in chests
      (bind _outactors_2 (`GameplayStatics.GetAllActorsOfClass` "/Game/Blueprints/BP_TreasureChest.BP_TreasureChest_C"))
      (for _array_element_2 _outactors_2
        (set `self.MaxCoinCount` (+ (`self.MaxCoinCount`) (`/Game/Blueprints/BP_TreasureChest.CoinsInChest` _array_element_2)))))
    (:`then_2`
      ;[1 1 1] Coins text widget
      (bind _returnvalue (`|GenericCreateObject` (`GameplayStatics.GetPlayerController` 0) "/Game/FirstPerson/Blueprints/WBP_CoinUI.WBP_CoinUI_C"))
      (bind _output_get (set `self.CoinText` _returnvalue))
      (`UserWidget.AddToViewport` _output_get 0))))

(event `CollectCoin`
  ;[1 1 1] Increment CoinCounter
  (`/Engine/EditorBlueprintResources/StandardMacros.IncrementInt` (`self.CoinCount`)
    (:`  `
      (`self.UpdateCoinUI` :!label _label))))

(event `LootChest`
  (params (CointAmount :type Integer))
  ;[1 1 1] Add multiple coins
  (set `self.CoinCount` (+ CointAmount (`self.CoinCount`)))
  (goto _label))

(fn `UpdateCoinUI`
  (bind _coincount (`self.CoinCount`))
  (`/Game/FirstPerson/Blueprints/WBP_CoinUI.UpdateCoinUI` (`self.CoinText`) _coincount)
  (if (>= _coincount (`self.MaxCoinCount`))
    (`KismetSystemLibrary.PrintString` "You got all the coins")
    (else
      (`KismetSystemLibrary.PrintString` "There are more coins to get"))))

(fn `UserConstructionScript`)