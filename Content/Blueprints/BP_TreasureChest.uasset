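; BP_TreasureChest is an interactable chest that opens its lid and awards coins to the player.
; Interact plays ChestTimeline, which rotates LidPivot around its roll axis by the negated timeline value.
; When the timeline finishes, an uncollected chest casts the game mode to GM_CoinCollector, calls LootChest with CoinsInChest and marks itself collected so it pays out only once.
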(event `/Game/Blueprints/Coin/BPI_Interactible.Interact`
  (bind (_direction _rotation) (`Timeline|ChestTimeline`)
    (:`Update`
      (`SceneComponent.K2_SetRelativeRotation` (`self.LidPivot`) (`KismetMathLibrary.MakeRotator` (* _rotation -1.0)) false false))
    (:`Finished`
      (if (not (`self.collected`))
        (bind _asgm_coin_collector (cast `/Game/Blueprints/Coin/GM_CoinCollector` (`GameplayStatics.GetGameMode`)))
        (`/Game/Blueprints/Coin/GM_CoinCollector.LootChest` _asgm_coin_collector (`self.CoinsInChest`))
        (set `self.collected` true)))))

(fn `UserConstructionScript`)